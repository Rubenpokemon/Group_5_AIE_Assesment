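; Enemy projectile actor that damages the first-person player on contact.
; On BeginPlay, a latent MoveComponentTo slides the Cube along X over the Speed duration, targeting its world X plus Distance as a relative location, then destroys the actor.
; An overlap on the Cube with FirstPersonCharacter calls its Hit function with a fixed damage value and destroys the bullet immediately.
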(event `self.ReceiveBeginPlay`
  (bind _cube (`self.Cube`))
  (bind _returnvalue_x (`KismetMathLibrary.BreakVector` (`SceneComponent.K2_GetComponentLocation` _cube)))
  (bind (_returnvalue_location _returnvalue_rotation) (`KismetMathLibrary.BreakTransform` (`SceneComponent.GetRelativeTransform` _cube)))
  (`KismetSystemLibrary.MoveComponentTo` _cube (`KismetMathLibrary.MakeVector` (+ _returnvalue_x (`self.Distance`))) _returnvalue_rotation false false (`self.Speed`))
  (`self.K2_DestroyActor`))

(event `self.Cube.OnComponentBeginOverlap`
  (params (OverlappedComponent :type "PrimitiveComponent Object Reference") (OtherActor :type "Actor Object Reference") (OtherComp :type "PrimitiveComponent Object Reference") (OtherBodyIndex :type Integer) (bFromSweep :type Boolean) (SweepResult :type "HitResult Structure (by ref)"))
  (bind _asfirst_person_character (cast `/Game/FirstPersonBP/Blueprints/FirstPersonCharacter` OtherActor))
  (`/Game/FirstPersonBP/Blueprints/FirstPersonCharacter.Hit` _asfirst_person_character 5)
  (`self.K2_DestroyActor`))

(fn `UserConstructionScript`)