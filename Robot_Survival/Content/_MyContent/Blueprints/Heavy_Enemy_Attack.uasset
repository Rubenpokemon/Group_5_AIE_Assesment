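; Heavy enemy attack actor: a moving cube that detects hits on the first-person player.
; On BeginPlay it slides the cube over a set time to a relative X built from its world X plus a distance, then destroys itself.
; Overlapping the FirstPersonCharacter during the move prints a hit message and destroys the actor early, with no damage applied.
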(event `self.ReceiveBeginPlay`
  (bind _cube (`self.Cube`))
  (bind _returnvalue_x (`KismetMathLibrary.BreakVector` (`SceneComponent.K2_GetComponentLocation` _cube)))
  (bind (_returnvalue_location _returnvalue_rotation) (`KismetMathLibrary.BreakTransform` (`SceneComponent.GetRelativeTransform` _cube)))
  (`KismetSystemLibrary.MoveComponentTo` _cube (`KismetMathLibrary.MakeVector` (+ _returnvalue_x (`self.Distance`))) _returnvalue_rotation false false (`self.Time`))
  (`self.K2_DestroyActor`))

(event `self.Cube.OnComponentBeginOverlap`
  (params (OverlappedComponent :type "PrimitiveComponent Object Reference") (OtherActor :type "Actor Object Reference") (OtherComp :type "PrimitiveComponent Object Reference") (OtherBodyIndex :type Integer) (bFromSweep :type Boolean) (SweepResult :type "HitResult Structure (by ref)"))
  (cast `/Game/FirstPersonBP/Blueprints/FirstPersonCharacter` OtherActor)
  (`KismetSystemLibrary.PrintString` "Player Hit By Heavy Attack")
  (`self.K2_DestroyActor`))

(fn `UserConstructionScript`)