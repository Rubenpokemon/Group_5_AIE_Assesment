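; Ranged enemy that chases the player and fires Enemy_Bullet, and is destroyed after enough FirstPersonProjectile hits deplete its Health.
; PawnSensing latches the first sighted player as target, and Tick reissues AIMoveTo toward it.
; Box overlap starts an attack loop that halts the enemy by disabling CharacterMovement tick, plays a timeline, spawns a bullet, then waits AttackSpeed.
; The loop repeats while the player stays in the box, otherwise movement resumes.
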(event `self.CapsuleComponent.OnComponentHit`
  (params (HitComponent :type "PrimitiveComponent Object Reference") (OtherActor :type "Actor Object Reference") (OtherComp :type "PrimitiveComponent Object Reference") (NormalImpulse :type "Vector Structure") (Hit :type "HitResult Structure (by ref)"))
  (cast `/Game/FirstPersonBP/Blueprints/FirstPersonProjectile` OtherActor)
  (`KismetSystemLibrary.PrintString` "Enemy Hit")
  (set `self.Health` (- (`self.Health`) 0.5))
  (if (<= (`self.Health`) 0.0)
    (`self.K2_DestroyActor`)))

(event `self.ReceiveTick`
  (params (DeltaSeconds :type "Float (single-precision)"))
  (if (`self.Moving`)
    (`|AIMoveTo` self (0.0 0.0 0.0) (`self.Player`))))

(event `self.PawnSensing.OnSeePawn`
  (params (Pawn :type "Pawn Object Reference"))
  (bind _asfirst_person_character (cast `/Game/FirstPersonBP/Blueprints/FirstPersonCharacter` Pawn))
  (if (not (`self.Moving`))
    (set `self.Moving` true)
    (set `self.Player` _asfirst_person_character)))

(event `self.Box.OnComponentBeginOverlap`
  (params (OverlappedComponent :type "PrimitiveComponent Object Reference") (OtherActor :type "Actor Object Reference") (OtherComp :type "PrimitiveComponent Object Reference") (OtherBodyIndex :type Integer) (bFromSweep :type Boolean) (SweepResult :type "HitResult Structure (by ref)"))
  (if (`ActorComponent.IsComponentTickEnabled` (`self.CharacterMovement`))
    (cast `/Game/FirstPersonBP/Blueprints/FirstPersonCharacter` OtherActor)
    (`self.Attack`)))

(event `Attack`
  (`ActorComponent.SetComponentTickEnabled` (`self.CharacterMovement`) false)
  (`Timeline|Attack_timeline`
    (:`Finished`
      (`self.Spawn_Attack`)
      (`KismetSystemLibrary.Delay` (`self.Attack Speed`))
      (if (`PrimitiveComponent.IsOverlappingActor` (`self.Box`) (`self.Player`))
        (`self.Attack`)
        (else
          (`ActorComponent.SetComponentTickEnabled` (`self.CharacterMovement`) true))))))

(event `Spawn_Attack`
  (bind (_returnvalue_x _returnvalue_y _returnvalue_z) (`KismetMathLibrary.BreakVector` (`self.K2_GetActorLocation` self)))
  (`|SpawnActorFromClass` "/Game/_MyContent/Blueprints/Enemy_Bullet.Enemy_Bullet_C" (`KismetMathLibrary.MakeTransform` (`KismetMathLibrary.MakeVector` _returnvalue_x _returnvalue_y _returnvalue_z) (`self.K2_GetActorRotation` self)) "Undefined" "OverrideRootScale" null null))

(fn `UserConstructionScript`)